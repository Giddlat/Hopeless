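; BP_Flag is the mini-golf hole flag, which moves out of the ball's way and triggers the win.
; Tick compares the golf pawn's sphere to the flag's starting position using the absolute sum of offset components, not true distance.
; Within the threshold a Timeline drives the flag mesh's relative Z, reversing otherwise.
; Any overlap with the flag's Sphere shows the WinState widget, then quits the game after a delay.
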(event OnComponentBeginOverlap(Sphere)
  (params (OverlappedComponent :type Primitive%20Component%20Object%20Reference) (OtherActor :type Actor%20Object%20Reference) (OtherComp :type Primitive%20Component%20Object%20Reference) (OtherBodyIndex :type Integer) (bFromSweep :type Boolean) (SweepResult :type Hit%20Result%20Structure%20%28by%20ref%29))
  ;[1 1 1] WinState
  (bind _returnvalue (UserInterface|CreateWidget "/Game/GAME/CrazyMiniGolf/UMG/WinState.WinState_C"))
  (UserInterface|Viewport|AddtoViewport _returnvalue 0)
  (Utilities|FlowControl|Delay 5.0)
  (Game|QuitGame (Game|GetPlayerController 0) "Quit"))

(event EventTick
  (params (DeltaSeconds :type Float%20%28single-precision%29))
  (bind _flag (Variables|Default|GetFlag))
  (bind _returnvalue (Transformation|GetRelativeTransform _flag))
  ;[1 1 1] Move The Flag
  (bind _asbp_golf_pawn (Utilities|Casting|CastToBP_GolfPawn (Game|Player|GetPlayerPawn 0)))
  (if (<= (Math|Float|Absolute(Float) (+ (.x (- (Transformation|GetWorldLocation (Variables|/Game/GAME/CrazyMiniGolf/Player/BP_GolfPawn.BP_GolfPawn_C|GetSphere _asbp_golf_pawn)) (Variables|Default|GetWorld%20Location))) (.y (- (Transformation|GetWorldLocation (Variables|/Game/GAME/CrazyMiniGolf/Player/BP_GolfPawn.BP_GolfPawn_C|GetSphere _asbp_golf_pawn)) (Variables|Default|GetWorld%20Location))) (.z (- (Transformation|GetWorldLocation (Variables|/Game/GAME/CrazyMiniGolf/Player/BP_GolfPawn.BP_GolfPawn_C|GetSphere _asbp_golf_pawn)) (Variables|Default|GetWorld%20Location))))) 4e+02)
    (bind _newtrack_0 (Timeline|Timeline_0 Play)
      (:Update
        (Transformation|SetRelativeLocation _flag (Math|Vector|MakeVector (.x (.location _returnvalue)) (.y (.location _returnvalue)) _newtrack_0) false false)))
    (else
      (Timeline|Timeline_0 Reverse))))

(event EventBeginPlay
  ;[1 1 1] Defining Variables
  (Variables|Default|SetWorld%20Location (Transformation|GetWorldLocation (Variables|Default|GetDefaultSceneRoot))))

(fn ConstructionScript)